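; BP_Team represents a team of heroes in the Lighthall game and relays game-flow and turn-flow events to its members.
; GameWillBegin is forwarded to every entry in the Heroes array.
; TurnWillBegin and TurnWillEnd are forwarded the same way, but only while the ActiveTeam flag is set, so an inactive team's heroes receive no turn events from it.
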(event EventGameWillBegin
  ;[1 0.1046 0.855] Game Flow
  (for _array_element (Variables|Default|GetHeroes)
    (Default|GameWillBegin _array_element)))

(event EventTurnWillBegin
  ;[1 0.1046 0.855] Turn Flow
  (if (Variables|Default|GetActiveTeam)
    (for _array_element (Variables|Default|GetHeroes)
      (Default|TurnWillBegin _array_element))))

(event EventTurnWillEnd
  ;[1 0.1046 0.855] Turn Flow
  (if (Variables|Default|GetActiveTeam)
    (for _array_element (Variables|Default|GetHeroes)
      (Default|TurnWillEnd _array_element))))

(fn ConstructionScript)