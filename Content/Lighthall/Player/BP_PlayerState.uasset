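; Player state that owns a player's team and relays game and turn lifecycle events.
; On load, the server spawns and registers a BP_Team, waits for replication, spawns four fixed heroes at the first area tagged by objective and team ID, waits again, then notifies the game mode.
; Lifecycle events forward through Client events to controller messages, with some also notifying the Team.
; Clients apply ally selection decals to their team's heroes.
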(event Custom|CreateTeam
  ;[1 1 1] Team Setup
  (bind _returnvalue (Game|SpawnActorfromClass "/Game/Lighthall/Game/BP_Team.BP_Team_C" (Math|Transform|MakeTransform "0, 0, 0") "AlwaysSpawn" self 0))
  (bind _output_get (Variables|Default|SetTeam _returnvalue))
  (bind _asgame_state_control (Utilities|Casting|CastToGameState_Control (Game|GetGameState)))
  (Utilities|Array|Add (Variables|/Game/Lighthall/Game/GameState_Control.GameState_Control_C|GetTeams _asgame_state_control) _output_get)
  (bind _result (Math|Integer|IncrementInt (Variables|/Game/Lighthall/Game/GameState_Control.GameState_Control_C|GetNumberOfTeams _asgame_state_control))
    (:%20%20
      (bind _output_get_2 (Variables|/Game/Lighthall/Game/BP_Team.BP_Team_C|SetTeamID _output_get _result))
      ;;[1 1 1] This makes Team1 the first active Team
      (Variables|/Game/Lighthall/Game/BP_Team.BP_Team_C|SetActiveTeam (Variables|Default|GetTeam) (== _output_get_2 1)))))

(event Custom|PrintClientTeamData
  (bind _team (Variables|Default|GetTeam))
  ;[1 1 1] Debug
  (if (not (Networking|IsServer))
    (bind _asgame_state_control (Utilities|Casting|CastToGameState_Control (Game|GetGameState)))
    (Development|PrintString (Utilities|String|Append " 
TeamID: " (Utilities|String|ToString(Integer) (Variables|/Game/Lighthall/Game/BP_Team.BP_Team_C|GetTeamID _team)) " 
Heroes: " (Utilities|String|ToString(Integer) (Utilities|Array|Length (Variables|/Game/Lighthall/Game/BP_Team.BP_Team_C|GetHeroes _team))) " 
Number of Teams: " (Utilities|String|ToString(Integer) (Utilities|Array|Length (Variables|/Game/Lighthall/Game/GameState_Control.GameState_Control_C|GetTeams _asgame_state_control))) " 
--------------------------") true true "(R=0.805844,G=1.000000,B=0.000000,A=1.000000)" 1e+02)))

(event Custom|ClientGameDidLoad
  ;[1 0.1046 0.855] Game Flow
  (Class|GameFlowObserver|GameDidLoad(Message) (Class|GameplayStatics|GetPlayerControllerfromID)))

(event Custom|ClientTurnWillEnd
  ;[1 0.1046 0.855] Turn Flow
  (Class|GameFlowObserver|TurnWillEnd(Message) (Class|GameplayStatics|GetPlayerControllerfromID)))

(event Custom|SetAllySelectionDecals
  ;[1 1 1] Team Setup
  (if (not (Networking|IsServer))
    ;;[0.3115 0.3115 1] The only heroes we can access client-side will be on your team
    (for _array_element (Variables|/Game/Lighthall/Game/BP_Team.BP_Team_C|GetHeroes (Variables|Default|GetTeam))
      (Rendering|Components|Decal|SetDecalMaterial (Variables|/Game/Lighthall/Hero/BP_HeroCharacter.BP_HeroCharacter_C|GetSelectionDecal _array_element) "/Game/Lighthall/Materials/M_SelectionDecal_Ally.M_SelectionDecal_Ally"))))

(event Custom|CreateTeamHeroes
  (bind _team (Variables|Default|GetTeam))
  (bind _teamid (Variables|/Game/Lighthall/Game/BP_Team.BP_Team_C|GetTeamID _team))
  ;[1 1 1] Team Setup
  (bind _outactors (Actor|GetAllActorsOfClasswithTag "/Game/Lighthall/Props/BP_SpawnArea.BP_SpawnArea_C" (Utilities|String|StringToName (CallFunction|SpawnAreaTag))))
  (bind _array_element (Utilities|Array|ForEachLoopwithBreak _outactors :!label _label)
    (:LoopBody
      (bind _hero (Default|SpawnNewHero _array_element "/Game/Lighthall/Hero/Heroes/Arryn/Hero_Arryn.Hero_Arryn_C" _teamid))
      (Utilities|Array|Add (Variables|/Game/Lighthall/Game/BP_Team.BP_Team_C|GetHeroes _team) _hero)
      (bind _hero_2 (Default|SpawnNewHero _array_element "/Game/Lighthall/Hero/Heroes/Eyliir/Hero_Eyliir.Hero_Eyliir_C" _teamid))
      (Utilities|Array|Add (Variables|/Game/Lighthall/Game/BP_Team.BP_Team_C|GetHeroes _team) _hero_2)
      (bind _hero_3 (Default|SpawnNewHero _array_element "/Game/Lighthall/Hero/Heroes/Kiri/Hero_Kiri.Hero_Kiri_C" _teamid))
      (Utilities|Array|Add (Variables|/Game/Lighthall/Game/BP_Team.BP_Team_C|GetHeroes _team) _hero_3)
      (bind _hero_4 (Default|SpawnNewHero _array_element "/Game/Lighthall/Hero/Heroes/River/Hero_River.Hero_River_C" _teamid))
      (Utilities|Array|Add (Variables|/Game/Lighthall/Game/BP_Team.BP_Team_C|GetHeroes _team) _hero_4)
      (goto _label Break))))

(event Custom|ClientTurnDidEnd
  ;[1 0.1046 0.855] Turn Flow
  (Class|GameFlowObserver|TurnDidEnd(Message) (Class|GameplayStatics|GetPlayerControllerfromID)))

(event Custom|ClientTurnDidBegin
  ;[1 0.1046 0.855] Turn Flow
  (Class|GameFlowObserver|TurnDidBegin(Message) (Class|GameplayStatics|GetPlayerControllerfromID)))

(event Custom|ClientTurnWillBegin
  ;[1 0.1046 0.855] Turn Flow
  (Class|GameFlowObserver|TurnWillBegin(Message) (Class|GameplayStatics|GetPlayerControllerfromID)))

(event Custom|ClientGameWillBegin
  ;[1 0.1046 0.855] Game Flow
  (Class|GameFlowObserver|GameWillBegin(Message) (Class|GameplayStatics|GetPlayerControllerfromID)))

(event Custom|ClientGameDidBegin
  ;[1 0.1046 0.855] Game Flow
  (Class|GameFlowObserver|GameDidBegin(Message) (Class|GameplayStatics|GetPlayerControllerfromID)))

(event EventTurnWillBegin
  ;[1 0.1046 0.855] Turn Flow
  (CallFunction|ClientTurnWillBegin)
  (Default|TurnWillBegin (Variables|Default|GetTeam)))

(event EventTurnDidBegin
  ;[1 0.1046 0.855] Turn Flow
  (CallFunction|ClientTurnDidBegin))

(event EventGameWillBegin
  ;[1 0.1046 0.855] Game Flow
  (CallFunction|ClientGameWillBegin)
  (Default|GameWillBegin (Variables|Default|GetTeam)))

(event EventTurnWillEnd
  ;[1 0.1046 0.855] Turn Flow
  (CallFunction|ClientTurnWillEnd)
  (Default|TurnWillEnd (Variables|Default|GetTeam)))

(event EventTurnDidEnd
  ;[1 0.1046 0.855] Turn Flow
  (CallFunction|ClientTurnDidEnd))

(event EventGameWillLoad
  ;[1 0.1046 0.855] Game Flow
  (if (Networking|IsServer)
    (CallFunction|CreateTeam)
    (Class|AutomationBlueprintFunctionLibrary|AutomationWaitforLoading (Utilities|Struct|MakeAutomationWaitForLoadingOptions true)) ; This ensures that Team is replicated to client before continuing
    (CallFunction|CreateTeamHeroes)
    (Class|AutomationBlueprintFunctionLibrary|AutomationWaitforLoading (Utilities|Struct|MakeAutomationWaitForLoadingOptions true)) ; This ensures that the team's heroes are replicated to client before continuing
    (bind _asgame_mode_control (Utilities|Casting|CastToGameMode_Control (Game|GetGameMode)))
    (Default|PlayerFinishedLoading _asgame_mode_control)))

(event EventGameDidLoad
  ;[1 0.1046 0.855] Game Flow
  (CallFunction|ClientGameDidLoad)
  (CallFunction|SetAllySelectionDecals))

(event EventGameDidBegin
  ;[1 0.1046 0.855] Game Flow
  (CallFunction|ClientGameDidBegin))

(fn ConstructionScript)

(fn SpawnAreaTag
  (bind _asgame_state_control (Utilities|Casting|CastToGameState_Control (Game|GetGameState)))
  (return (Utilities|String|Append (Variables|/Game/Lighthall/Game/GameState_Control.GameState_Control_C|GetCurrentObjectiveTag _asgame_state_control) (Utilities|String|ToString(Integer) (Variables|/Game/Lighthall/Game/BP_Team.BP_Team_C|GetTeamID (Variables|Default|GetTeam))))))