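; Base hero ability actor that runs a use pipeline: play the caster's animation, set cooldown, apply effects, then notify its observer.
; Effects are copied onto the target's Afflictions or Curatives, stamped with the source hero.
; Targeting capsule-traces around the caster and attaches decals to valid heroes by ability type.
; Client-only cosmetics cover cooldown updates and particles, though the attached-particle path is disconnected.
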(event Custom|Init
  (params (SlotID :type Integer) (Observer :type BPI%20Ability%20Observer%20Interface%20%28by%20ref%29))
  (Variables|Appearance|SetSlotID SlotID)
  (Variables|Observers|SetAbilityObserver Observer))

(event Custom|PostExecute
  (params (TargetHero :type BP%20Hero%20Character%20Object%20Reference%20%28by%20ref%29) (SourceHero :type BP%20Hero%20Character%20Object%20Reference%20%28by%20ref%29) (TargetLocation :type Vector))
  (Variables|/Game/Lighthall/Hero/BP_HeroCharacter.BP_HeroCharacter_C|SetUsedAbility SourceHero true)
  (Default|AbilityUsed (Variables|Observers|GetAbilityObserver) self))

(event Custom|PreExecute
  (params (TargetHero :type BP%20Hero%20Character%20Object%20Reference%20%28by%20ref%29) (SourceHero :type BP%20Hero%20Character%20Object%20Reference%20%28by%20ref%29) (TargetLocation :type Vector))
  (bind _duration (Default|AnimateHero SourceHero (Variables|Behavior|GetExecuteAnimation) TargetLocation))
  (Utilities|FlowControl|Delay _duration)
  (CallFunction|Execute TargetHero SourceHero TargetLocation))

(event Custom|MulticastDecrementCooldown
  (Variables|Behavior|SetRemainingCooldown (+ (Variables|Behavior|GetCooldown) 1))
  (if (not (Networking|IsServer))
    (bind _asbp_hero_character (Utilities|Casting|CastToBP_HeroCharacter (Actor|GetParentActor)))
    (Default|UpdatedAbilityCooldown _asbp_hero_character)))

(event Custom|Execute
  (params (TargetHero :type BP%20Hero%20Character%20Object%20Reference%20%28by%20ref%29) (SourceHero :type BP%20Hero%20Character%20Object%20Reference%20%28by%20ref%29) (TargetLocation :type Vector))
  (CallFunction|MulticastDecrementCooldown)
  (if (or (Utilities|Enum|Equal(Enum) (Variables|Behavior|GetType) "NewEnumerator3") (Utilities|IsValid TargetHero))
    (CallFunction|GiveTargetEffects TargetHero SourceHero)
    (CallFunction|PostExecute TargetHero SourceHero TargetLocation)))

(event Custom|TargetValidHeroes
  (params (SourceHero :type BP%20Hero%20Character%20Object%20Reference))
  (bind _returnvalue (Transformation|GetActorLocation SourceHero))
  (bind _range (Variables|Behavior|GetRange))
  (bind _outhits (Class|KismetSystemLibrary|CapsuleTraceMultiforObjects (+ _returnvalue _range) (- _returnvalue _range) _range (Variables|/Script/Engine.CapsuleComponent|GetCapsuleHalfHeight (Variables|/Script/Engine.Character|GetCapsuleComponent SourceHero)) (Utilities|Array|MakeArray (Utilities|Enum|LiteralenumEObjectTypeQuery "ObjectTypeQuery3")) true 0 "Persistent" true "(R=1.000000,G=1.000000,B=1.000000,A=1.000000)" "(R=0.000000,G=1.000000,B=0.000000,A=1.000000)" 1e+01))
  (for _array_element _outhits
    (bind _asbp_hero_character (Utilities|Casting|CastToBP_HeroCharacter (.hitactor _array_element)))
    (if (Default|IsValidTarget SourceHero _asbp_hero_character self "0, 0, 0")
      (switch Utilities|FlowControl|Switch|SwitchonEffectType (Variables|Behavior|GetType)
        (:NewEnumerator0
          (bind _returnvalue_2 (Class|GameplayStatics|SpawnDecalAttached "/Game/Lighthall/Materials/M_AbilityTargetDecal_Damage.M_AbilityTargetDecal_Damage" (Math|Vector|MakeVector (.x (Variables|/Script/Engine.DecalComponent|GetDecalSize (Variables|/Game/Lighthall/Hero/BP_HeroCharacter.BP_HeroCharacter_C|GetSelectionDecal _asbp_hero_character))) (.y (Variables|/Script/Engine.DecalComponent|GetDecalSize (Variables|/Game/Lighthall/Hero/BP_HeroCharacter.BP_HeroCharacter_C|GetSelectionDecal _asbp_hero_character))) (.z (Variables|/Script/Engine.DecalComponent|GetDecalSize (Variables|/Game/Lighthall/Hero/BP_HeroCharacter.BP_HeroCharacter_C|GetSelectionDecal _asbp_hero_character)))) (Variables|/Script/Engine.Character|GetCapsuleComponent _asbp_hero_character) "None" "0, 0, 0" "-90.000000,0.000000, 0" "KeepRelativeOffset" 0.0))
          (Variables|/Game/Lighthall/Hero/BP_HeroCharacter.BP_HeroCharacter_C|SetTargetDecal _asbp_hero_character _returnvalue_2))
        (:NewEnumerator1
          (bind _returnvalue_3 (Class|GameplayStatics|SpawnDecalAttached "/Game/Lighthall/Materials/M_AbilityTargetDecal_Heal.M_AbilityTargetDecal_Heal" (Math|Vector|MakeVector (.x (Variables|/Script/Engine.DecalComponent|GetDecalSize (Variables|/Game/Lighthall/Hero/BP_HeroCharacter.BP_HeroCharacter_C|GetSelectionDecal _asbp_hero_character))) (.y (Variables|/Script/Engine.DecalComponent|GetDecalSize (Variables|/Game/Lighthall/Hero/BP_HeroCharacter.BP_HeroCharacter_C|GetSelectionDecal _asbp_hero_character))) (.z (Variables|/Script/Engine.DecalComponent|GetDecalSize (Variables|/Game/Lighthall/Hero/BP_HeroCharacter.BP_HeroCharacter_C|GetSelectionDecal _asbp_hero_character)))) (Variables|/Script/Engine.Character|GetCapsuleComponent _asbp_hero_character) "None" "0, 0, 0" "-90.000000,0.000000, 0" "KeepRelativeOffset" 0.0 :!label _label))
          (Variables|/Game/Lighthall/Hero/BP_HeroCharacter.BP_HeroCharacter_C|SetTargetDecal _asbp_hero_character _returnvalue_3))
        (:NewEnumerator4
          (goto _label))
        (:NewEnumerator2
          (goto _label))
        (:NewEnumerator3
          (bind _returnvalue_4 (Class|GameplayStatics|SpawnDecalAttached "/Game/Lighthall/Materials/M_AbilityTargetDecal_Neutral.M_AbilityTargetDecal_Neutral" (Math|Vector|MakeVector (.x (Variables|/Script/Engine.DecalComponent|GetDecalSize (Variables|/Game/Lighthall/Hero/BP_HeroCharacter.BP_HeroCharacter_C|GetSelectionDecal _asbp_hero_character))) (.y (Variables|/Script/Engine.DecalComponent|GetDecalSize (Variables|/Game/Lighthall/Hero/BP_HeroCharacter.BP_HeroCharacter_C|GetSelectionDecal _asbp_hero_character))) (.z (Variables|/Script/Engine.DecalComponent|GetDecalSize (Variables|/Game/Lighthall/Hero/BP_HeroCharacter.BP_HeroCharacter_C|GetSelectionDecal _asbp_hero_character)))) (Variables|/Script/Engine.Character|GetCapsuleComponent _asbp_hero_character) "None" "0, 0, 0" "-90.000000,0.000000, 0" "KeepRelativeOffset" 0.0))
          (Variables|/Game/Lighthall/Hero/BP_HeroCharacter.BP_HeroCharacter_C|SetTargetDecal _asbp_hero_character _returnvalue_4))))))

(event Custom|Use
  (params (TargetHero :type BP%20Hero%20Character%20Object%20Reference%20%28by%20ref%29) (SourceHero :type BP%20Hero%20Character%20Object%20Reference%20%28by%20ref%29) (TargetLocation :type Vector))
  (CallFunction|PreExecute TargetHero SourceHero TargetLocation))

(event Custom|MulticastAbilityParticles
  (params (Particles :type Particle%20System%20Object%20Reference) (MaxDuration :type Float%20%28single-precision%29) (Attached :type Boolean) (Offset :type Vector) (Scale :type Vector))
  (if (not (Networking|IsServer))
    (if (not Attached)
      (bind _returnvalue (Effects|SpawnEmitteratLocation Particles (Transformation|GetActorLocation) "0, 0, 0" Scale true "AutoRelease"))
      (if (> MaxDuration 0.0)
        (Utilities|FlowControl|Delay MaxDuration)
        (Components|DestroyComponent _returnvalue)))))

(event Custom|UntargetAllHeroes
  (bind _outactors (Actor|GetAllActorsOfClass "/Game/Lighthall/Hero/BP_HeroCharacter.BP_HeroCharacter_C"))
  (for _array_element _outactors
    (Components|DestroyComponent (Variables|/Game/Lighthall/Hero/BP_HeroCharacter.BP_HeroCharacter_C|GetTargetDecal _array_element))))

(fn ConstructionScript)

(fn GiveTargetEffects
  (params (TargetHero :type BP%20Hero%20Character%20Object%20Reference) (SourceHero :type BP%20Hero%20Character%20Object%20Reference))
  (for _array_element (Variables|Behavior|GetEffects)
    (if (Utilities|Enum|Equal(Enum) (.effecttype _array_element) "NewEnumerator0")
      (Utilities|Array|Add (Variables|/Game/Lighthall/Hero/BP_HeroCharacter.BP_HeroCharacter_C|GetAfflictions TargetHero) (Utilities|Struct|MakeEffect (.effecttype _array_element) (.name _array_element) (.description _array_element) (.emblem _array_element) (.healthmutation _array_element) (.status _array_element) (.duration _array_element) SourceHero))
      (else
        (Utilities|Array|Add (Variables|/Game/Lighthall/Hero/BP_HeroCharacter.BP_HeroCharacter_C|GetCuratives TargetHero) (Utilities|Struct|MakeEffect (.effecttype _array_element) (.name _array_element) (.description _array_element) (.emblem _array_element) (.healthmutation _array_element) (.status _array_element) (.duration _array_element) SourceHero))))))