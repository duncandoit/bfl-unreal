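; Spawn area prop that creates new heroes with a team ID or teleports existing heroes back into the area.
; Both use a random transform within the scaled Bounds extents on world X/Y, ignoring area rotation, at the Bounds' height with random yaw.
; New spawns adjust for collisions but always succeed.
; The construction script labels SpawnTitle from the first two characters of an actor tag, read as spawn point and team.
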(event Custom|ReturnHeroToSpawn
  (params (Hero :type BP%20Hero%20Character%20Object%20Reference%20%28by%20ref%29))
  (bind _location (CallFunction|RandomSpawnTransform))
  (Transformation|Teleport Hero (.location _location) (.rotation _location)))

(fn ConstructionScript
  (for _array_element (Variables|Actor|GetTags)
    (Rendering|Components|TextRender|SetText (Variables|Default|GetSpawnTitle) (Utilities|Text|ToText(String) (Utilities|String|Append "Spawn 
" "Point " (Utilities|String|GetSubstring (Utilities|String|ToString(Name) _array_element) 0) ", Team " (Utilities|String|GetSubstring (Utilities|String|ToString(Name) _array_element) 1))))))

(fn RandomSpawnTransform
  (bind _bounds (Variables|Default|GetBounds))
  (bind _returnvalue (Transformation|GetWorldTransform _bounds))
  (bind _max (Components|StaticMesh|GetLocalBounds _bounds))
  (bind _returnvalue_2 (Transformation|GetWorldLocation _bounds))
  (bind _returnvalue_3 (* (.x _max) (.x (.scale _returnvalue))))
  (bind _returnvalue_4 (* (.y _max) (.y (.scale _returnvalue))))
  (return (Math|Transform|MakeTransform (Math|Vector|MakeVector (Math|Random|RandomFloatinRange (- (.x _returnvalue_2) _returnvalue_3) (+ (.x _returnvalue_2) _returnvalue_3)) (Math|Random|RandomFloatinRange (- (.y _returnvalue_2) _returnvalue_4) (+ (.y _returnvalue_2) _returnvalue_4)) (.z _returnvalue_2)) (Math|Rotator|MakeRotator 0.0 0.0 (Math|Random|RandomFloatinRange 0.0 3.6e+02)))))

(fn SpawnNewHero
  (params (HeroClass :type BP%20Hero%20Character%20Class%20Reference) (Team :type Integer))
  (bind _returnvalue (Game|SpawnActorfromClass HeroClass (CallFunction|RandomSpawnTransform) "AdjustIfPossibleButAlwaysSpawn" 0 0))
  (Variables|/Game/Lighthall/Hero/BP_HeroCharacter.BP_HeroCharacter_C|SetTeamID _returnvalue Team)
  (return _returnvalue))